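; BP_MazeCell is a configurable maze cell actor, assembled entirely in its construction script.
; It scales SMCube as the floor slab from Gridsize, deriving wall thickness as a fraction of that size.
; Per-side flags add scaled static mesh walls, and a Ceiling flag adds a top slab.
; Ceilinged cells also get a centered, colored point light below the ceiling when the light intensity is above zero.
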(fn `UserConstructionScript`
  (locals (Wallthickness :type "Float (double-precision)" :default 1.0) (Walllength :type "Float (double-precision)" :default 1.0))
  (bind _gridsize (`self.Gridsize`))
  (bind _walllength (`local.Walllength`))
  (bind _walllength_2 (`local.Walllength`))
  (bind _returnvalue (* (`local.Walllength`) 0.5))
  (set `local.Walllength` _gridsize)
  (set `local.Wallthickness` (* _gridsize 0.1))
  (`SceneComponent.SetRelativeScale3D` (`self.SM_Cube`) (`self.NewMacro` (`KismetMathLibrary.MakeVector` _walllength_2 _walllength_2 (`local.Wallthickness`))))
  (if (`self.westwall`)
    (`AddComponent|NODE_AddStaticMeshComponent-0` :`RelativeTransform` (`KismetMathLibrary.MakeTransform` (0.0 0.0 0.0) (struct) (`self.NewMacro` (`KismetMathLibrary.MakeVector` (`local.Walllength`) (`local.Wallthickness`) (`self.wallheight`))))))
  (if (`self.Southwall`)
    (`AddComponent|NODE_AddStaticMeshComponent-1` :`RelativeTransform` (`KismetMathLibrary.MakeTransform` (0.0 0.0 0.0) (struct) (`self.NewMacro` (`KismetMathLibrary.MakeVector` (`local.Wallthickness`) (`local.Walllength`) (`self.wallheight`))))))
  (if (`self.Northwall`)
    (`AddComponent|NODE_AddStaticMeshComponent-3` :`RelativeTransform` (`KismetMathLibrary.MakeTransform` (`KismetMathLibrary.MakeVector` (- (`local.Walllength`) (`local.Wallthickness`))) (struct) (`self.NewMacro` (`KismetMathLibrary.MakeVector` (`local.Wallthickness`) (`local.Walllength`) (`self.wallheight`))))))
  (if (`self.eastwall`)
    (`AddComponent|NODE_AddStaticMeshComponent-4` :`RelativeTransform` (`KismetMathLibrary.MakeTransform` (`KismetMathLibrary.MakeVector` 0.0 (- (`local.Walllength`) (`local.Wallthickness`))) (struct) (`self.NewMacro` (`KismetMathLibrary.MakeVector` (`local.Walllength`) (`local.Wallthickness`) (`self.wallheight`))))))
  (if (`self.Ceiling`)
    (`AddComponent|NODE_AddStaticMeshComponent-5` :`RelativeTransform` (`KismetMathLibrary.MakeTransform` (`KismetMathLibrary.MakeVector` 0.0 0.0 (`self.wallheight`)) (struct) (`self.NewMacro` (`KismetMathLibrary.MakeVector` _walllength _walllength (`local.Wallthickness`)))))
    (if (> (`self.lightensity`) 0.0)
      (bind _returnvalue_2 (`AddComponent|NODE_AddPointLightComponent-0` :`RelativeTransform` (`KismetMathLibrary.MakeTransform` (`KismetMathLibrary.MakeVector` _returnvalue _returnvalue (* (`self.wallheight`) 0.9)))))
      (`LightComponent.SetLightColor` _returnvalue_2 (`self.New Light Color`) true)
      (`LightComponent.SetIntensity` _returnvalue_2 (`self.lightensity`)))))